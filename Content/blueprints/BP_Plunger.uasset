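; BP_Plunger is a plunger actor that pulls its mesh back while charging and snaps it back on release.
; ChargePlunger plays a timeline whose alpha lerps PlungerMesh along its local Y axis from the rest position.
; StopCharge stops the timeline and uses MoveComponentTo to quickly return the mesh.
; GetBallSpawnLocation converts the BallLocation offset to world space through the actor's transform.
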(event `Charge Plunger`
  (bind (_direction _charge_alpha) (`Timeline|ChargeTimeline` :!label _label)
    (:`Update`
      (`SceneComponent.K2_SetRelativeLocation` (`self.PlungerMesh`) (`KismetMathLibrary.VLerp` (0.0 0.0 0.0) (0.0 150.0 0.0) _charge_alpha) false false))))

(event `Stop Charge`
  (`|ExecutionSequence`
    (:`then_0`
      (goto _label :!via `Stop`))
    (:`then_1`
      (`KismetSystemLibrary.MoveComponentTo` (`self.PlungerMesh`) (0.0 0.0 0.0) (struct) false false 0.05))))

(fn `GetBallSpawnLocation`
  (returns (BallSpawnLoc :type "Vector Structure"))
  (return (`KismetMathLibrary.TransformLocation` (`self.GetTransform`) (`self.BallLocation`))))

(fn `UserConstructionScript`)