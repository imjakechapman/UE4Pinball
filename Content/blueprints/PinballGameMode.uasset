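; Pinball game mode that runs the game flow from main menu through ball play to game over, tracking score, multiplier and balls left.
; Reset restores class defaults and spawns a ball at the plunger; each ball's destruction triggers a respawn until none remain.
; Game end checks a lazily loaded, cached high-score save to show either the score-entry widget or the game-over menu.
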(event `self.ReceiveBeginPlay`
  (`self.CreateMainMenu`))

(event `CreateMainMenu`
  (bind _aspinball_player_controller (cast `/Game/blueprints/PinballPlayerController` (`GameplayStatics.GetPlayerController` 0) :!pure true))
  (`self.GetGameSaveData`)
  (`WidgetLayoutLibrary.RemoveAllWidgets`)
  (bind _returnvalue (`|CreateWidget` "/Game/blueprints/MainMenu.MainMenu_C" _aspinball_player_controller))
  (`UserWidget.AddToViewport` _returnvalue 0)
  (set `PlayerController.bShowMouseCursor` true _aspinball_player_controller))

(event `ResetGame`
  (bind (_score _multiplier _ballsleft) (defaults `/Game/blueprints/PinballGameMode` "PinballGameMode_C"))
  (bind _aspinball_player_controller (cast `/Game/blueprints/PinballPlayerController` (`GameplayStatics.GetPlayerController` 0) :!pure true))
  (`WidgetLayoutLibrary.RemoveAllWidgets`)
  (set `self.Score` _score)
  (set `self.Multiplier` _multiplier)
  (set `self.BallsLeft` _ballsleft)
  (`GameplayStatics.PlaySound2D` "/Game/assets/sounds/GameStartCue.GameStartCue")
  (`self.SpawnBall`)
  (`/Game/blueprints/PinballPlayerController.CreatePlayerHUD` _aspinball_player_controller)
  (set `PlayerController.bShowMouseCursor` false _aspinball_player_controller))

(event `SpawnBall`
  (bind _outactors (`GameplayStatics.GetAllActorsOfClass` "/Game/blueprints/BP_Plunger.BP_Plunger_C"))
  (`GameplayStatics.PlaySound2D` "/Game/assets/sounds/PinballResetCue.PinballResetCue")
  (bind _returnvalue (`|SpawnActorFromClass` "/Game/blueprints/BP_Ball.BP_Ball_C" (`KismetMathLibrary.MakeTransform` (`/Game/blueprints/BP_Plunger.GetBallSpawnLocation` (`|GetArrayItem` _outactors))) "Undefined" "OverrideRootScale" null null))
  (add `self.OnDestroyed` _returnvalue (delegate `OnBallDestroyed`)))

(event `OnBallDestroyed` :!signature `self.OnDestroyed`
  (params (DestroyedActor :type "Actor Object Reference"))
  (if (<= (`self.BallsLeft`) 0)
    (`self.EndGame`)
    (else
      (`/Engine/EditorBlueprintResources/StandardMacros.DecrementInt` (`self.BallsLeft`)
        (:`  `
          (`self.SpawnBall`))))))

(event `EndGame`
  (bind _currentsaveobject (`self.GetGameSaveData`))
  (if (<= (`KismetArrayLibrary.Array_Length` (`/Game/blueprints/HighScoreSave.SaveStruct` _currentsaveobject)) 3)
    (`self.CreateHighScoresList` :!label _label)
    (else
      (bind _lowest_score_struct (`/Game/blueprints/HighScoreSave.CheckLowestScore` _currentsaveobject))
      (if (< (`.Score_5_1700D43D4C4025658250AC85737F63A6` (break `/Game/blueprints/HighscoreStruct` _lowest_score_struct)) (`self.Score`))
        (goto _label)
        (else
          (`self.CreateGameOverScreen`))))))

(event `CreateHighScoresList`
  (bind _aspinball_player_controller (cast `/Game/blueprints/PinballPlayerController` (`GameplayStatics.GetPlayerController` 0) :!pure true))
  (bind _returnvalue (`|CreateWidget` "/Game/blueprints/HighScoreEntry.HighScoreEntry_C" _aspinball_player_controller))
  (`UserWidget.AddToViewport` _returnvalue 0)
  (set `PlayerController.bShowMouseCursor` true _aspinball_player_controller))

(event `CreateGameOverScreen`
  (bind _aspinball_player_controller (cast `/Game/blueprints/PinballPlayerController` (`GameplayStatics.GetPlayerController` 0) :!pure true))
  (`WidgetLayoutLibrary.RemoveAllWidgets`)
  (bind _returnvalue (`|CreateWidget` "/Game/blueprints/GameOverMenu.GameOverMenu_C" _aspinball_player_controller))
  (`UserWidget.AddToViewport` _returnvalue 0)
  (set `PlayerController.bShowMouseCursor` true _aspinball_player_controller))

(fn `AddScore`
  (params (PointsToAdd :type "Float (double-precision)"))
  (returns (NewScore :type "Float (double-precision)"))
  (bind _output_get (set `self.Score` (+ (* PointsToAdd (`self.Multiplier`)) (`self.Score`))))
  (return _output_get))

(fn `GetGameSaveData`
  (returns (CurrentSaveObject :type "/Game/blueprints/HighScoreSave Object Reference"))
  (bind _currentsaveobject (`self.CurrentSaveObject`)
    (:`then`
      (return _currentsaveobject))
    (:`else`
      (bind _returnvalue (`GameplayStatics.DoesSaveGameExist` (`self.HighscoreSaveName`)))
      (if _returnvalue
        (bind _returnvalue_2 (`GameplayStatics.LoadGameFromSlot` (`self.HighscoreSaveName`)))
        (bind _ashigh_score_save (cast `/Game/blueprints/HighScoreSave` _returnvalue_2)
          (:`then`
            (`/Game/blueprints/HighScoreSave.SortSaveData` _ashigh_score_save)
            (bind _output_get (set `self.CurrentSaveObject` _ashigh_score_save))
            (return _output_get))
          (:`CastFailed`
            (return null)))
        (else
          (bind _returnvalue_3 (`GameplayStatics.CreateSaveGameObject` "/Game/blueprints/HighScoreSave.HighScoreSave_C"))
          (bind _output_get_2 (set `self.CurrentSaveObject` _returnvalue_3))
          (return _output_get_2))))))

(fn `UserConstructionScript`)